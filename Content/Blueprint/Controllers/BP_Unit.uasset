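; Selectable grid unit that occupies a tile on BP_Grid and travels along tile paths.
; After a short startup delay it finds the grid, snaps to the nearest tile and registers as its occupant.
; Clicks on its capsule or cones toggle selection through BP_PlayerController.
; For movement it updates tile occupancy upfront, rebuilds the grid's shared spline from the path, and follows it via timeline while flagging the grid busy.
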(event OnClicked(Cone1)
  (params (TouchedComponent :type Primitive%20Component%20Object%20Reference) (ButtonPressed :type Key%20Structure :default "None"))
  (if (!= (Variables|/Game/Blueprint/Controllers/BP_PlayerController.BP_PlayerController_C|GetSelectedUnit (Variables|Default|GetplayerController)) self)
    (Default|EventNewUnitSelected (Variables|Default|GetplayerController) self)
    (CallFunction|EventSelected)
    (else
      (Default|EventNewUnitSelected (Variables|Default|GetplayerController)))))

(event OnClicked(Cone)
  (params (TouchedComponent :type Primitive%20Component%20Object%20Reference) (ButtonPressed :type Key%20Structure :default "None"))
  (if (!= (Variables|/Game/Blueprint/Controllers/BP_PlayerController.BP_PlayerController_C|GetSelectedUnit (Variables|Default|GetplayerController)) self)
    (Default|EventNewUnitSelected (Variables|Default|GetplayerController) self)
    (CallFunction|EventSelected)
    (else
      (Default|EventNewUnitSelected (Variables|Default|GetplayerController)))))

(event OnClicked(CapsuleComponent)
  (params (TouchedComponent :type Primitive%20Component%20Object%20Reference) (ButtonPressed :type Key%20Structure :default "None"))
  (if (!= (Variables|/Game/Blueprint/Controllers/BP_PlayerController.BP_PlayerController_C|GetSelectedUnit (Variables|Default|GetplayerController)) self)
    (Default|EventNewUnitSelected (Variables|Default|GetplayerController) self)
    (CallFunction|EventSelected)
    (else
      (Default|EventNewUnitSelected (Variables|Default|GetplayerController)))))

(event Custom|Event_Selected
  (Development|PrintString "Selected"))

(event Custom|Event_Deselected
  (Development|PrintString "DeSelected"))

(event Custom|Event_MoveAlongThePath
  (params (path :type Array%20of%20Vector%202D%20Structures))
  (bind _grid (Variables|Default|GetGrid))
  (bind _spline (Variables|/Game/Blueprint/Grid/BP_Grid.BP_Grid_C|GetSpline _grid))
  (Variables|Default|SetPath path)
  (Utilities|Array|Insert (Variables|Default|GetPath) (Variables|Default|GetgridIndex))
  (CallFunction|UnitonThisTile (Utilities|Array|Get(acopy) (Variables|Default|GetPath) (Utilities|Array|LastIndex (Variables|Default|GetPath))))
  (Spline|ClearSplinePoints (Variables|/Game/Blueprint/Grid/BP_Grid.BP_Grid_C|GetSpline (Variables|Default|GetGrid)) true)
  (for _array_element (Variables|Default|GetPath)
    (Spline|AddSplinePoint (Variables|/Game/Blueprint/Grid/BP_Grid.BP_Grid_C|GetSpline (Variables|Default|GetGrid)) (Math|Vector|MakeVector (.x (.worldlocation (.Value (Utilities|Map|Find (Variables|/Game/Blueprint/Grid/BP_Grid.BP_Grid_C|Getstruct_Tiles (Variables|Default|GetGrid)) _array_element)))) (.y (.worldlocation (.Value (Utilities|Map|Find (Variables|/Game/Blueprint/Grid/BP_Grid.BP_Grid_C|Getstruct_Tiles (Variables|Default|GetGrid)) _array_element)))) (+ (.z (.worldlocation (.Value (Utilities|Map|Find (Variables|/Game/Blueprint/Grid/BP_Grid.BP_Grid_C|Getstruct_Tiles (Variables|Default|GetGrid)) _array_element)))) (Variables|/Script/Engine.CapsuleComponent|GetCapsuleHalfHeight (Variables|Collision|GetCapsuleComponent)))) "Local" true))
  (Variables|/Game/Blueprint/Grid/BP_Grid.BP_Grid_C|SetbIsAUnitMoving (Variables|Default|GetGrid) true)
  (bind _progession (Timeline|MoveAlongThePathFindToTarget PlayFromStart)
    (:Update
      (Transformation|SetActorTransform (Math|Transform|MakeTransform (Spline|GetLocationatDistanceAlongSpline _spline (* _progession (Spline|GetSplineLength _spline)) "Local") (Spline|GetRotationatDistanceAlongSpline _spline (* _progession (Spline|GetSplineLength _spline)) "Local") "1,1,1")))
    (:Finished
      (Variables|/Game/Blueprint/Grid/BP_Grid.BP_Grid_C|SetbIsAUnitMoving (Variables|Default|GetGrid) false))))

(event EventBeginPlay
  (Utilities|FlowControl|Delay 1.0)
  (bind _asbp_player_controller (Utilities|Casting|CastToBP_PlayerController (Game|GetPlayerController 0)))
  (Variables|Default|SetplayerController _asbp_player_controller)
  (bind _outactors (Actor|GetAllActorsOfClass "/Game/Blueprint/Grid/BP_Grid.BP_Grid_C"))
  (if (Utilities|Array|IsValidIndex _outactors)
    (Variables|Default|SetGrid (Utilities|Array|Get(acopy) _outactors))
    (CallFunction|SetGridIndexandSnaptoLocation)))

(fn ConstructionScript)

(fn SetGridIndexandSnaptoLocation
  (LocalVariables|SetclosedDistance 1e+09)
  (bind _keys (Utilities|Map|Keys (Variables|/Game/Blueprint/Grid/BP_Grid.BP_Grid_C|Getstruct_Tiles (Variables|Default|GetGrid))))
  (for _array_element _keys
    (if (< (Math|Vector|VectorLength (- (.worldlocation (.Value (Utilities|Map|Find (Variables|/Game/Blueprint/Grid/BP_Grid.BP_Grid_C|Getstruct_Tiles (Variables|Default|GetGrid)) _array_element))) (Transformation|GetActorLocation))) (LocalVariables|GetclosedDistance))
      (LocalVariables|SetclosedDistance (Math|Vector|VectorLength (- (.worldlocation (.Value (Utilities|Map|Find (Variables|/Game/Blueprint/Grid/BP_Grid.BP_Grid_C|Getstruct_Tiles (Variables|Default|GetGrid)) _array_element))) (Transformation|GetActorLocation))))
      (LocalVariables|SetclosestIndex _array_element)))
  (CallFunction|UnitonThisTile (LocalVariables|GetclosestIndex))
  (Transformation|SetActorLocation (.worldlocation (.Value (Utilities|Map|Find (Variables|/Game/Blueprint/Grid/BP_Grid.BP_Grid_C|Getstruct_Tiles (Variables|Default|GetGrid)) (LocalVariables|GetclosestIndex)))) false false))

(fn UnitonThisTile
  (params (gridIndex :type Vector%202D%20Structure))
  (bind _grid (Variables|Default|GetGrid))
  (bind _grid_2 (Variables|Default|GetGrid))
  (bind _struct_tiles (Variables|/Game/Blueprint/Grid/BP_Grid.BP_Grid_C|Getstruct_Tiles _grid))
  (bind _struct_tiles_2 (Variables|/Game/Blueprint/Grid/BP_Grid.BP_Grid_C|Getstruct_Tiles _grid_2))
  (Utilities|Map|Add _struct_tiles_2 (Variables|Default|GetgridIndex) (Utilities|Struct|MakeStruct_Tiles (.tileactor (.Value (Utilities|Map|Find _struct_tiles_2 (Variables|Default|GetgridIndex)))) 0 (.groundtype (.Value (Utilities|Map|Find _struct_tiles_2 (Variables|Default|GetgridIndex)))) (.worldlocation (.Value (Utilities|Map|Find _struct_tiles_2 (Variables|Default|GetgridIndex)))) (.gridindex (.Value (Utilities|Map|Find _struct_tiles_2 (Variables|Default|GetgridIndex)))) (.tilecost (.Value (Utilities|Map|Find _struct_tiles_2 (Variables|Default|GetgridIndex)))) (.finalcost (.Value (Utilities|Map|Find _struct_tiles_2 (Variables|Default|GetgridIndex)))) (.costfromstart (.Value (Utilities|Map|Find _struct_tiles_2 (Variables|Default|GetgridIndex)))) (.estimatedcosttotarget (.Value (Utilities|Map|Find _struct_tiles_2 (Variables|Default|GetgridIndex)))) (.previoustile (.Value (Utilities|Map|Find _struct_tiles_2 (Variables|Default|GetgridIndex))))))
  (Variables|Default|SetgridIndex gridIndex)
  (Utilities|Map|Add _struct_tiles (Variables|Default|GetgridIndex) (Utilities|Struct|MakeStruct_Tiles (.tileactor (.Value (Utilities|Map|Find _struct_tiles (Variables|Default|GetgridIndex)))) self (.groundtype (.Value (Utilities|Map|Find _struct_tiles (Variables|Default|GetgridIndex)))) (.worldlocation (.Value (Utilities|Map|Find _struct_tiles (Variables|Default|GetgridIndex)))) (.gridindex (.Value (Utilities|Map|Find _struct_tiles (Variables|Default|GetgridIndex)))) (.tilecost (.Value (Utilities|Map|Find _struct_tiles (Variables|Default|GetgridIndex)))) (.finalcost (.Value (Utilities|Map|Find _struct_tiles (Variables|Default|GetgridIndex)))) (.costfromstart (.Value (Utilities|Map|Find _struct_tiles (Variables|Default|GetgridIndex)))) (.estimatedcosttotarget (.Value (Utilities|Map|Find _struct_tiles (Variables|Default|GetgridIndex)))) (.previoustile (.Value (Utilities|Map|Find _struct_tiles (Variables|Default|GetgridIndex)))))))