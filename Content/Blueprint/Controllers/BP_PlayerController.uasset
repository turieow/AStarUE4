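; Player controller that tracks the selected unit and relays movement paths to it.
; A new-selection event deselects the previous unit and stores the new one, while a new-path event tells the current unit to move along the supplied path.
; Holding R hides every BP_Base_Obstacle actor in the level, found by a class search on each press and release, and releasing it shows them again.
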(event Custom|Event_NewUnitSelected
  (params (Unit :type BP%20Unit%20Object%20Reference))
  (Utilities|IsValid (Variables|Default|GetSelectedUnit)
    (:Is%20Valid
      (Default|EventDeselected (Variables|Default|GetSelectedUnit)))
    (:Is%20Not%20Valid
      _))
  (Variables|Default|SetSelectedUnit Unit))

(event Custom|Event_NewPathAvillable
  (params (path :type Array%20of%20Vector%202D%20Structures))
  (bind _selectedunit (Variables|Default|GetSelectedUnit))
  (Utilities|IsValid _selectedunit
    (:Is%20Valid
      (Default|EventMoveAlongthePath _selectedunit path))))

(event Input|KeyboardEvents|R
  (params (Key :type Key%20Structure :default "None"))
  (:Pressed
    (bind _outactors (Actor|GetAllActorsOfClass "/Game/Blueprint/Grid/BP_Base_Obstacle.BP_Base_Obstacle_C"))
    (for _array_element _outactors
      (Rendering|SetActorHiddenInGame _array_element true)))
  (:Released
    (bind _outactors_2 (Actor|GetAllActorsOfClass "/Game/Blueprint/Grid/BP_Base_Obstacle.BP_Base_Obstacle_C"))
    (for _array_element_2 _outactors_2
      (Rendering|SetActorHiddenInGame _array_element_2 false))))

(fn ConstructionScript)