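; BP_Grid is a tile grid actor that finds and highlights a path between the selected and hovered tiles.
; Sphere traces classify terrain and BP_Base_Obstacle ground types into a tile map, debug-drawn on construction.
; BeginPlay spawns BP_GridTile actors, whose selection and hover events trigger four-way, A*-style pathfinding with terrain costs.
; Hover runs the debug search event, whose neighbour heuristic measures to the start tile; the FindPathToTarget function is unwired.
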(event Custom|Event_NewTileSelected
  (params (selecttile :type BP%20Grid%20Tile%20Object%20Reference))
  (Utilities|IsValid (Variables|グリッド|GetSelecterTile)
    (:Is%20Valid
      (Default|EventDeselectTile (Variables|グリッド|GetSelecterTile)))
    (:Is%20Not%20Valid
      _))
  (Variables|グリッド|SetSelecterTile selecttile))

(event Custom|Event_NewTileOvered
  (params (OveredTile :type BP%20Grid%20Tile%20Object%20Reference))
  (bind _selectertile (Variables|グリッド|GetSelecterTile))
  (Utilities|IsValid (Variables|グリッド|GetoveredTile)
    (:Is%20Valid
      (Default|EventEndOverTile (Variables|グリッド|GetoveredTile)))
    (:Is%20Not%20Valid
      _))
  (Variables|グリッド|SetoveredTile OveredTile)
  (CallFunction|HighlightCurrentPath false)
  (if (and (Utilities|IsValid _selectertile) (Utilities|IsValid (Variables|グリッド|GetoveredTile)))
    (CallFunction|DebugEventFindPathtoTarget (Variables|/Game/Blueprint/Grid/BP_GridTile.BP_GridTile_C|Getgridindex _selectertile) (Variables|/Game/Blueprint/Grid/BP_GridTile.BP_GridTile_C|Getgridindex (Variables|グリッド|GetoveredTile)))
    (CallFunction|HighlightCurrentPath true)))

(event Custom|DebugEvent_FindPathToTarget
  (params (DebugStartTile :type Vector%202D%20Structure) (DebugTargetTile :type Vector%202D%20Structure))
  (bind _struct_tiles (Variables|Default|Getstruct_Tiles))
  (bind _struct_tiles_2 (Variables|Default|Getstruct_Tiles))
  (Variables|Default|SetDebugStartTileL DebugStartTile)
  (Variables|Default|SetDebugTargetTIleL DebugTargetTile)
  (Utilities|Array|Clear (Variables|Default|GetDebugOpenSet))
  (Utilities|Array|Clear (Variables|Default|GetDebugCloseSet))
  (Utilities|Array|Clear (Variables|Default|GetPath))
  (Variables|Default|SetDebugJobCompleted false)
  (if (Math|Boolean|ANDBoolean (.ReturnValue (Utilities|Map|Find (Variables|Default|Getstruct_Tiles) (Variables|Default|GetDebugTargetTIleL))) (Utilities|Enum|NotEqual(Enum) (.groundtype (.Value (Utilities|Map|Find (Variables|Default|Getstruct_Tiles) (Variables|Default|GetDebugTargetTIleL)))) "NewEnumerator4") (Utilities|Enum|NotEqual(Enum) (.groundtype (.Value (Utilities|Map|Find (Variables|Default|Getstruct_Tiles) (Variables|Default|GetDebugTargetTIleL)))) "NewEnumerator3"))
    (Utilities|FlowControl|Sequence
      (:then_0
        ;[1 1 1] コメント
        (bind _keys (Utilities|Map|Keys (Variables|Default|Getstruct_Tiles)))
        (for _array_element _keys
          (Utilities|Map|Add (Variables|Default|Getstruct_Tiles) _array_element (Utilities|Struct|MakeStruct_Tiles (.tileactor (.Value (Utilities|Map|Find (Variables|Default|Getstruct_Tiles) _array_element))) (.groundtype (.Value (Utilities|Map|Find (Variables|Default|Getstruct_Tiles) _array_element))) (.worldlocation (.Value (Utilities|Map|Find (Variables|Default|Getstruct_Tiles) _array_element))) (.gridindex (.Value (Utilities|Map|Find (Variables|Default|Getstruct_Tiles) _array_element))) (.tilecost (.Value (Utilities|Map|Find (Variables|Default|Getstruct_Tiles) _array_element))) 999 999 999 "(X=0.000000,Y=0.000000)")))
        (Utilities|Map|Add (Variables|Default|Getstruct_Tiles) (Variables|Default|GetDebugStartTileL) (Utilities|Struct|MakeStruct_Tiles (.tileactor (.Value (Utilities|Map|Find (Variables|Default|Getstruct_Tiles) (Variables|Default|GetDebugStartTileL)))) (.groundtype (.Value (Utilities|Map|Find (Variables|Default|Getstruct_Tiles) (Variables|Default|GetDebugStartTileL)))) (.worldlocation (.Value (Utilities|Map|Find (Variables|Default|Getstruct_Tiles) (Variables|Default|GetDebugStartTileL)))) (.gridindex (.Value (Utilities|Map|Find (Variables|Default|Getstruct_Tiles) (Variables|Default|GetDebugStartTileL)))) (.tilecost (.Value (Utilities|Map|Find (Variables|Default|Getstruct_Tiles) (Variables|Default|GetDebugStartTileL)))) (パスファインダー|GetEstimatedCosttoTarget (Variables|Default|GetDebugStartTileL) (Variables|Default|GetDebugTargetTIleL)) 0 (パスファインダー|GetEstimatedCosttoTarget (Variables|Default|GetDebugStartTileL) (Variables|Default|GetDebugTargetTIleL)) "(X=0.000000,Y=0.000000)")))
      (:then_1
        (Variables|Default|SetDebugCurrentTile (Variables|Default|GetDebugStartTileL))
        (Utilities|Array|AddUnique (Variables|Default|GetDebugOpenSet) (Variables|Default|GetDebugStartTileL))
        (while (and (> (Utilities|Array|Length (Variables|Default|GetDebugOpenSet)) 0) (not (Variables|Default|GetDebugJobCompleted)))
          (Variables|Default|SetDebugOpenSetCheapest (Utilities|Array|Get(acopy) (Variables|Default|GetDebugOpenSet)))
          (for _array_element_2 (Variables|Default|GetDebugOpenSet)
            (if (< (.finalcost (.Value (Utilities|Map|Find _struct_tiles _array_element_2))) (.finalcost (.Value (Utilities|Map|Find _struct_tiles (Variables|Default|GetDebugOpenSetCheapest)))))
              (Variables|Default|SetDebugOpenSetCheapest _array_element_2 :!label _label)
              (elif (== (.finalcost (.Value (Utilities|Map|Find _struct_tiles _array_element_2))) (.finalcost (.Value (Utilities|Map|Find _struct_tiles (Variables|Default|GetDebugOpenSetCheapest)))))
                (if (< (.estimatedcosttotarget (.Value (Utilities|Map|Find _struct_tiles _array_element_2))) (.estimatedcosttotarget (.Value (Utilities|Map|Find _struct_tiles (Variables|Default|GetDebugOpenSetCheapest)))))
                  (goto _label)))))
          (Variables|Default|SetDebugCurrentTile (Variables|Default|GetDebugOpenSetCheapest))
          (Utilities|Array|RemoveItem (Variables|Default|GetDebugOpenSet) (Variables|Default|GetDebugCurrentTile))
          (Utilities|Array|AddUnique (Variables|Default|GetDebugCloseSet) (Variables|Default|GetDebugCurrentTile))
          (for _array_element_3 (パスファインダー|GetTileNeighbours (Variables|Default|GetDebugCurrentTile))
            (Variables|Default|SetDebugCurrentNeightbour _array_element_3)
            (if (not (Utilities|Array|ContainsItem (Variables|Default|GetDebugCloseSet) (Variables|Default|GetDebugCurrentNeightbour)))
              (Variables|Default|SetDebugCurrentNeighbourCostFromStart (+ (.costfromstart (.Value (Utilities|Map|Find (Variables|Default|Getstruct_Tiles) (Variables|Default|GetDebugCurrentTile)))) (.tilecost (.Value (Utilities|Map|Find (Variables|Default|Getstruct_Tiles) (Variables|Default|GetDebugCurrentTile))))))
              (if (not (Utilities|Array|ContainsItem (Variables|Default|GetDebugOpenSet) (Variables|Default|GetDebugCurrentNeightbour)))
                (Utilities|Array|AddUnique (Variables|Default|GetDebugOpenSet) (Variables|Default|GetDebugCurrentNeightbour))
                (Utilities|Map|Add _struct_tiles_2 (Variables|Default|GetDebugCurrentNeightbour) (Utilities|Struct|MakeStruct_Tiles (.tileactor (.Value (Utilities|Map|Find _struct_tiles_2 (Variables|Default|GetDebugCurrentNeightbour)))) (.groundtype (.Value (Utilities|Map|Find _struct_tiles_2 (Variables|Default|GetDebugCurrentNeightbour)))) (.worldlocation (.Value (Utilities|Map|Find _struct_tiles_2 (Variables|Default|GetDebugCurrentNeightbour)))) (.gridindex (.Value (Utilities|Map|Find _struct_tiles_2 (Variables|Default|GetDebugCurrentNeightbour)))) (.tilecost (.Value (Utilities|Map|Find _struct_tiles_2 (Variables|Default|GetDebugCurrentNeightbour)))) (+ (Variables|Default|GetDebugCurrentNeighbourCostFromStart) (パスファインダー|GetEstimatedCosttoTarget (Variables|Default|GetDebugCurrentNeightbour) (Variables|Default|GetDebugStartTileL))) (Variables|Default|GetDebugCurrentNeighbourCostFromStart) (パスファインダー|GetEstimatedCosttoTarget (Variables|Default|GetDebugCurrentNeightbour) (Variables|Default|GetDebugStartTileL)) (Variables|Default|GetDebugCurrentTile)) :!label _label_2)
                (if (Math|Vector|Equal(Vector) (Variables|Default|GetDebugCurrentNeightbour) (Variables|Default|GetDebugTargetTIleL) 0.0001)
                  (Variables|Default|SetPath (パスファインダー|RetracePath (Variables|Default|GetDebugTargetTIleL) (Variables|Default|GetDebugStartTileL)))
                  (Variables|Default|SetDebugJobCompleted true))
                (elif (< (Variables|Default|GetDebugCurrentNeighbourCostFromStart) (.costfromstart (.Value (Utilities|Map|Find _struct_tiles_2 (Variables|Default|GetDebugCurrentNeightbour)))))
                  (goto _label_2))))))
        (if (Variables|Default|GetDebugJobCompleted)
          (CallFunction|HighlightCurrentPath true)
          (else
            (Development|PrintString "Fail")))))))

(event EventBeginPlay
  (Rendering|Debug|FlushPersistentDebugLines)
  (Variables|Grid|SetGridLocation (Transformation|GetWorldLocation (Variables|Default|GetBillboard)))
  (グリッド|GenerateMapDatafromWorld)
  (デバッグ|SpawnTile false))

(fn ConstructionScript
  (bind _gridsizeworld (Variables|グリッド|GetGridSizeWorld))
  (Rendering|Debug|FlushPersistentDebugLines)
  (Variables|Grid|SetGridLocation (Transformation|GetWorldLocation (Variables|Default|GetBillboard)))
  (Rendering|Debug|DrawDebugBox (Variables|Grid|GetGridLocation) (Math|Vector|MakeVector (.y _gridsizeworld) (.x _gridsizeworld) 5.0) (Variables|Debug|GetGridBoxColor) "0, 0, 0" 1e+05 1e+01)
  (Rendering|Debug|DrawDebugBox (グリッド|GridBottomLeft) (Math|Vector|MakeVector 2e+01 2e+01 2e+01) (Variables|デバッグ|GetBottomLeftColor) "0, 0, 0" 1e+05 1e+01)
  (グリッド|GenerateMapDatafromWorld)
  (Debug|DrawTile))

(fn GridBottomLeft
  (return (- (- (Variables|Grid|GetGridLocation) (* (Math|Vector|GetRightVector (Variables|Default|GetScene)) (.x (Variables|グリッド|GetGridSizeWorld)))) (* (Math|Vector|GetForwardVector (Variables|Default|GetScene)) (.y (Variables|グリッド|GetGridSizeWorld))))))

(fn GridTileNumber
  (bind _gridsizeworld (Variables|グリッド|GetGridSizeWorld))
  (bind _tilesize (Variables|グリッド|GetTileSize))
  (bind _returnvalue (/ _gridsizeworld _tilesize))
  (return (- (Math|Float|Round (.x _returnvalue)) 1) (- (Math|Float|Round (.y _returnvalue)) 1)))

(fn DrawTile
  (bind _keys (Utilities|Map|Keys (Variables|Default|Getstruct_Tiles)))
  (for _array_element _keys
    (デバッグ|MyDrawDebugPlane (.worldlocation (.Value (Utilities|Map|Find (Variables|Default|Getstruct_Tiles) _array_element))) (.groundtype (.Value (Utilities|Map|Find (Variables|Default|Getstruct_Tiles) _array_element))))))

(fn MySphereTrace
  (params (Location :type Vector) (TraceChannel :type ETraceTypeQuery%20Enum :default "TraceTypeQuery3"))
  (bind (_outhit _returnvalue) (Collision|SphereTraceByChannel Location Location (- (Variables|グリッド|GetTileSize) (Variables|グリッド|GetTileSizeMinus)) TraceChannel false 0 "None" true "(R=1.000000,G=0.000000,B=0.000000,A=1.000000)" "(R=0.000000,G=1.000000,B=0.000000,A=1.000000)" 1e+05))
  (return _returnvalue (.hitactor _outhit)))

(fn MyDrawDebugPlane
  (params (InVec :type Vector) (GroundType :type Enum_GroundType%20Enum :default "NewEnumerator0"))
  (switch Utilities|FlowControl|Switch|SwitchonEnum_GroundType GroundType
    (:NewEnumerator0
      (LocalVariables|SetTyleColor "(R=0.845772,G=1.000000,B=0.808946,A=1.000000)"))
    (:NewEnumerator1
      (LocalVariables|SetTyleColor "(R=0.101052,G=0.712500,B=0.097559,A=1.000000)"))
    (:NewEnumerator2
      (LocalVariables|SetTyleColor "(R=0.795833,G=0.328400,B=0.000000,A=1.000000)"))
    (:NewEnumerator3
      (LocalVariables|SetTyleColor "(R=1.000000,G=0.000000,B=0.094805,A=1.000000)")))
  (Class|KismetSystemLibrary|DrawDebugPlane (Utilities|Struct|MakePlane (.Z (Math|Vector|BreakVector InVec)) 0.0 0.0 1.0) InVec (- (Variables|グリッド|GetTileSize) (Variables|グリッド|GetTileSizeMinus)) (LocalVariables|GetTyleColor) 1e+05))

(fn GenerateMapDatafromWorld
  (bind (_gridtilenumberx _gridtilenumbery) (Grid|GridTileNumber))
  (bind _tilesize (Variables|グリッド|GetTileSize))
  (bind _tilesize_2 (Variables|グリッド|GetTileSize))
  (for _index (range 0 _gridtilenumberx)
    (LocalVariables|SetX _index)
    (for _index_2 (range 0 _gridtilenumbery)
      (LocalVariables|SetY _index_2)
      (LocalVariables|SetTilePosition (+ (グリッド|GridBottomLeft) (* (Math|Vector|GetRightVector (Variables|Default|GetScene)) (+ (* (LocalVariables|GetX) (* 2 _tilesize_2)) _tilesize_2)) (* (Math|Vector|GetForwardVector (Variables|Default|GetScene)) (+ (* (LocalVariables|GetY) (* 2 _tilesize)) _tilesize))))
      (if (.HitSomesthing (グリッド|MySphereTrace (LocalVariables|GetTilePosition) "TraceTypeQuery3"))
        (if (.HitSomesthing (グリッド|MySphereTrace (LocalVariables|GetTilePosition) "TraceTypeQuery4"))
          (Utilities|Map|Add (Variables|Default|Getstruct_Tiles) (Math|Vector2D|MakeVector2D (Math|Conversions|ToFloat(Integer) (LocalVariables|GetX)) (Math|Conversions|ToFloat(Integer) (LocalVariables|GetY))) (Utilities|Struct|MakeStruct_Tiles 0 (Variables|/Game/Blueprint/Grid/BP_Base_Obstacle.BP_Base_Obstacle_C|GetEnum_GroundTypes (.AsBP%20Base%20Obstacle (Utilities|Casting|CastToBP_Base_Obstacle (.Actor (グリッド|MySphereTrace (LocalVariables|GetTilePosition) "TraceTypeQuery4"))))) (LocalVariables|GetTilePosition) (Math|Vector2D|MakeVector2D (Math|Conversions|ToFloat(Integer) (LocalVariables|GetX)) (Math|Conversions|ToFloat(Integer) (LocalVariables|GetY))) (グリッド|GetTileCost (Variables|/Game/Blueprint/Grid/BP_Base_Obstacle.BP_Base_Obstacle_C|GetEnum_GroundTypes (.AsBP%20Base%20Obstacle (Utilities|Casting|CastToBP_Base_Obstacle (.Actor (グリッド|MySphereTrace (LocalVariables|GetTilePosition) "TraceTypeQuery4")))))) 0 0 0 "(X=0.000000,Y=0.000000)"))
          (else
            (Utilities|Map|Add (Variables|Default|Getstruct_Tiles) (Math|Vector2D|MakeVector2D (Math|Conversions|ToFloat(Integer) (LocalVariables|GetX)) (Math|Conversions|ToFloat(Integer) (LocalVariables|GetY))) (Utilities|Struct|MakeStruct_Tiles 0 "NewEnumerator0" (LocalVariables|GetTilePosition) (Math|Vector2D|MakeVector2D (Math|Conversions|ToFloat(Integer) (LocalVariables|GetX)) (Math|Conversions|ToFloat(Integer) (LocalVariables|GetY))) (グリッド|GetTileCost "NewEnumerator0") 0 0 0 "(X=0.000000,Y=0.000000)"))))
        (else
          (Utilities|Map|Add (Variables|Default|Getstruct_Tiles) (Math|Vector2D|MakeVector2D (Math|Conversions|ToFloat(Integer) (LocalVariables|GetX)) (Math|Conversions|ToFloat(Integer) (LocalVariables|GetY))) (Utilities|Struct|MakeStruct_Tiles 0 "NewEnumerator4" (LocalVariables|GetTilePosition) (Math|Vector2D|MakeVector2D (Math|Conversions|ToFloat(Integer) (LocalVariables|GetX)) (Math|Conversions|ToFloat(Integer) (LocalVariables|GetY))) (グリッド|GetTileCost "NewEnumerator4") 0 0 0 "(X=0.000000,Y=0.000000)")))))))

(fn SpawnTile
  (params (SpawnNoneTile :type Boolean))
  (bind _struct_tiles (Variables|Default|Getstruct_Tiles))
  (bind _keys (Utilities|Map|Keys (Variables|Default|Getstruct_Tiles)))
  (for _array_element _keys
    (if (or (Utilities|Enum|NotEqual(Enum) (.groundtype (.Value (Utilities|Map|Find _struct_tiles _array_element))) "NewEnumerator4") SpawnNoneTile)
      (bind _returnvalue (Game|SpawnActorfromClass "/Game/Blueprint/Grid/BP_GridTile.BP_GridTile_C" (Math|Conversions|ToTransform(Vector) (.worldlocation (.Value (Utilities|Map|Find _struct_tiles _array_element)))) "Undefined" 0 0))
      (Variables|/Game/Blueprint/Grid/BP_GridTile.BP_GridTile_C|Setgridindex _returnvalue (.gridindex (.Value (Utilities|Map|Find _struct_tiles _array_element))))
      (Variables|/Game/Blueprint/Grid/BP_GridTile.BP_GridTile_C|Setbp_Grid _returnvalue self)
      (Utilities|Map|Add _struct_tiles _array_element (Utilities|Struct|MakeStruct_Tiles _returnvalue (.groundtype (.Value (Utilities|Map|Find _struct_tiles _array_element))) (.worldlocation (.Value (Utilities|Map|Find _struct_tiles _array_element))) (.gridindex (.Value (Utilities|Map|Find _struct_tiles _array_element))) (.tilecost (.Value (Utilities|Map|Find _struct_tiles _array_element))) (.finalcost (.Value (Utilities|Map|Find _struct_tiles _array_element))) (.costfromstart (.Value (Utilities|Map|Find _struct_tiles _array_element))) (.estimatedcosttotarget (.Value (Utilities|Map|Find _struct_tiles _array_element))) (.previoustile (.Value (Utilities|Map|Find _struct_tiles _array_element))))))))

(fn GetTileCost
  (params (gridIndex :type Enum_GroundType%20Enum :default "NewEnumerator0"))
  (switch Utilities|FlowControl|Switch|SwitchonEnum_GroundType gridIndex
    (:NewEnumerator0
      (LocalVariables|SetCost 1))
    (:NewEnumerator1
      (LocalVariables|SetCost 2))
    (:NewEnumerator2
      (LocalVariables|SetCost 5))
    (:NewEnumerator3
      (LocalVariables|SetCost 999)))
  (return (LocalVariables|GetCost)))

(fn GetTileNeighbours
  (params (gridindex :type Vector%202D%20Structure))
  (bind _output_get (LocalVariables|SetpossibleNeighbours (Utilities|Array|MakeArray "(X=1.000000,Y=0.000000)" "(X=0.000000,Y=1.000000)" "(X=-1.000000,Y=0.000000)" "(X=0.000000,Y=-1.000000)")))
  (for _array_element _output_get
    (if (.ReturnValue (Utilities|Map|Find (Variables|Default|Getstruct_Tiles) (+ _array_element gridindex)))
      (if (and (Utilities|Enum|NotEqual(Enum) (.groundtype (.Value (Utilities|Map|Find (Variables|Default|Getstruct_Tiles) (+ _array_element gridindex)))) "NewEnumerator4") (Utilities|Enum|NotEqual(Enum) (.groundtype (.Value (Utilities|Map|Find (Variables|Default|Getstruct_Tiles) (+ _array_element gridindex)))) "NewEnumerator3"))
        (Utilities|Array|AddUnique (LocalVariables|GetoutNeighbours) (+ _array_element gridindex)))))
  (return (LocalVariables|GetoutNeighbours)))

(fn GetEstimatedCosttoTarget
  (params (currentTile :type Vector%202D%20Structure) (targetTile :type Vector%202D%20Structure))
  (bind _returnvalue (- currentTile targetTile))
  (return (Math|Float|Round (+ (Math|Float|Absolute(Float) (.x _returnvalue)) (Math|Float|Absolute(Float) (.y _returnvalue))))))

(fn FindPathtoTarget
  (params (StartTile :type Vector%202D%20Structure) (TargetTile :type Vector%202D%20Structure))
  (bind _struct_tiles (Variables|Default|Getstruct_Tiles))
  (bind _struct_tiles_2 (Variables|Default|Getstruct_Tiles))
  (LocalVariables|SetstartTileL StartTile)
  (LocalVariables|SetTargetTileL TargetTile)
  (if (Math|Boolean|ANDBoolean (.ReturnValue (Utilities|Map|Find (Variables|Default|Getstruct_Tiles) (LocalVariables|GetTargetTileL))) (Utilities|Enum|NotEqual(Enum) (.groundtype (.Value (Utilities|Map|Find (Variables|Default|Getstruct_Tiles) (LocalVariables|GetTargetTileL)))) "NewEnumerator4") (Utilities|Enum|NotEqual(Enum) (.groundtype (.Value (Utilities|Map|Find (Variables|Default|Getstruct_Tiles) (LocalVariables|GetTargetTileL)))) "NewEnumerator3"))
    (Utilities|FlowControl|Sequence
      (:then_0
        ;[1 1 1] コメント
        (bind _keys (Utilities|Map|Keys (Variables|Default|Getstruct_Tiles)))
        (for _array_element _keys
          (Utilities|Map|Add (Variables|Default|Getstruct_Tiles) _array_element (Utilities|Struct|MakeStruct_Tiles (.tileactor (.Value (Utilities|Map|Find (Variables|Default|Getstruct_Tiles) _array_element))) (.groundtype (.Value (Utilities|Map|Find (Variables|Default|Getstruct_Tiles) _array_element))) (.worldlocation (.Value (Utilities|Map|Find (Variables|Default|Getstruct_Tiles) _array_element))) (.gridindex (.Value (Utilities|Map|Find (Variables|Default|Getstruct_Tiles) _array_element))) (.tilecost (.Value (Utilities|Map|Find (Variables|Default|Getstruct_Tiles) _array_element))) 999 999 999 "(X=0.000000,Y=0.000000)")))
        (Utilities|Map|Add (Variables|Default|Getstruct_Tiles) (LocalVariables|GetstartTileL) (Utilities|Struct|MakeStruct_Tiles (.tileactor (.Value (Utilities|Map|Find (Variables|Default|Getstruct_Tiles) (LocalVariables|GetstartTileL)))) (.groundtype (.Value (Utilities|Map|Find (Variables|Default|Getstruct_Tiles) (LocalVariables|GetstartTileL)))) (.worldlocation (.Value (Utilities|Map|Find (Variables|Default|Getstruct_Tiles) (LocalVariables|GetstartTileL)))) (.gridindex (.Value (Utilities|Map|Find (Variables|Default|Getstruct_Tiles) (LocalVariables|GetstartTileL)))) (.tilecost (.Value (Utilities|Map|Find (Variables|Default|Getstruct_Tiles) (LocalVariables|GetstartTileL)))) (パスファインダー|GetEstimatedCosttoTarget (LocalVariables|GetstartTileL) (LocalVariables|GetTargetTileL)) 0 (パスファインダー|GetEstimatedCosttoTarget (LocalVariables|GetstartTileL) (LocalVariables|GetTargetTileL)) "(X=0.000000,Y=0.000000)")))
      (:then_1
        (LocalVariables|SetcurrentTile (LocalVariables|GetstartTileL))
        (Utilities|Array|AddUnique (LocalVariables|GetopenSet) (LocalVariables|GetstartTileL))
        (while (> (Utilities|Array|Length (LocalVariables|GetopenSet)) 0)
          (LocalVariables|SetopenSetCheapest (Utilities|Array|Get(acopy) (LocalVariables|GetopenSet)))
          (for _array_element_2 (LocalVariables|GetopenSet)
            (if (< (.finalcost (.Value (Utilities|Map|Find _struct_tiles _array_element_2))) (.finalcost (.Value (Utilities|Map|Find _struct_tiles (LocalVariables|GetopenSetCheapest)))))
              (LocalVariables|SetopenSetCheapest _array_element_2 :!label _label)
              (elif (== (.finalcost (.Value (Utilities|Map|Find _struct_tiles _array_element_2))) (.finalcost (.Value (Utilities|Map|Find _struct_tiles (LocalVariables|GetopenSetCheapest)))))
                (if (< (.estimatedcosttotarget (.Value (Utilities|Map|Find _struct_tiles _array_element_2))) (.estimatedcosttotarget (.Value (Utilities|Map|Find _struct_tiles (LocalVariables|GetopenSetCheapest)))))
                  (goto _label)))))
          (LocalVariables|SetcurrentTile (LocalVariables|GetopenSetCheapest))
          (Utilities|Array|RemoveItem (LocalVariables|GetopenSet) (LocalVariables|GetcurrentTile))
          (Utilities|Array|AddUnique (LocalVariables|GetcloseSet) (LocalVariables|GetcurrentTile))
          (for _array_element_3 (パスファインダー|GetTileNeighbours (LocalVariables|GetcurrentTile))
            (LocalVariables|SetcurrentNeighbour _array_element_3)
            (if (not (Utilities|Array|ContainsItem (LocalVariables|GetcloseSet) (LocalVariables|GetcurrentNeighbour)))
              (LocalVariables|SetcurrentNeighbourCostFromStart (+ (.costfromstart (.Value (Utilities|Map|Find (Variables|Default|Getstruct_Tiles) (LocalVariables|GetcurrentTile)))) (.tilecost (.Value (Utilities|Map|Find (Variables|Default|Getstruct_Tiles) (LocalVariables|GetcurrentNeighbour))))))
              (if (not (Utilities|Array|ContainsItem (LocalVariables|GetopenSet) (LocalVariables|GetcurrentNeighbour)))
                (Utilities|Array|AddUnique (LocalVariables|GetopenSet) (LocalVariables|GetcurrentNeighbour))
                (Utilities|Map|Add _struct_tiles_2 (LocalVariables|GetcurrentNeighbour) (Utilities|Struct|MakeStruct_Tiles (.tileactor (.Value (Utilities|Map|Find _struct_tiles_2 (LocalVariables|GetcurrentNeighbour)))) (.groundtype (.Value (Utilities|Map|Find _struct_tiles_2 (LocalVariables|GetcurrentNeighbour)))) (.worldlocation (.Value (Utilities|Map|Find _struct_tiles_2 (LocalVariables|GetcurrentNeighbour)))) (.gridindex (.Value (Utilities|Map|Find _struct_tiles_2 (LocalVariables|GetcurrentNeighbour)))) (.tilecost (.Value (Utilities|Map|Find _struct_tiles_2 (LocalVariables|GetcurrentNeighbour)))) (+ (LocalVariables|GetcurrentNeighbourCostFromStart) (パスファインダー|GetEstimatedCosttoTarget (LocalVariables|GetcurrentNeighbour) (LocalVariables|GetTargetTileL))) (LocalVariables|GetcurrentNeighbourCostFromStart) (パスファインダー|GetEstimatedCosttoTarget (LocalVariables|GetcurrentNeighbour) (LocalVariables|GetTargetTileL)) (LocalVariables|GetcurrentTile)) :!label _label_2)
                (if (Math|Vector|Equal(Vector) (LocalVariables|GetcurrentNeighbour) (LocalVariables|GetTargetTileL) 0.0001)
                  (Variables|Default|SetPath (パスファインダー|RetracePath (LocalVariables|GetTargetTileL) (LocalVariables|GetstartTileL)))
                  (return))
                (elif (< (LocalVariables|GetcurrentNeighbourCostFromStart) (.costfromstart (.Value (Utilities|Map|Find _struct_tiles_2 (LocalVariables|GetcurrentNeighbour)))))
                  (goto _label_2))))))
        ;[1 1 1] Fail
        (return)))))

(fn RetracePath
  (params (TargetTile :type Vector%202D%20Structure) (StartTile :type Vector%202D%20Structure))
  (LocalVariables|SetCurrentTile TargetTile)
  (while (Math|Vector|NotEqual(Vector) (LocalVariables|GetCurrentTile) StartTile 0.0001)
    (Utilities|Array|AddUnique (LocalVariables|GetinvertedPath) (LocalVariables|GetCurrentTile))
    (LocalVariables|SetCurrentTile (.previoustile (.Value (Utilities|Map|Find (Variables|Default|Getstruct_Tiles) (LocalVariables|GetCurrentTile))))))
  (bind _arrayelement (Utilities|Array|ReverseforEachLoop (LocalVariables|GetinvertedPath))
    (:LoopBody
      (Utilities|Array|AddUnique (LocalVariables|GetoutPath) _arrayelement))
    (:Completed
      (return (LocalVariables|GetoutPath)))))

(fn HighlightCurrentPath
  (params (isforHightlight :type Boolean))
  (for _array_element (Variables|Default|GetPath)
    (Utilities|IsValid (.tileactor (.Value (Utilities|Map|Find (Variables|Default|Getstruct_Tiles) _array_element)))
      (:Is%20Valid
        (Default|EventIsinPath (.tileactor (.Value (Utilities|Map|Find (Variables|Default|Getstruct_Tiles) _array_element))) isforHightlight)))))