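; Grid tile actor that displays its ground type and reports cursor hover and clicks to its owning BpGrid.
; It looks up its data in the grid's tile map by index, scales its cube to the grid's tile size and initializes a W_GridTile widget.
; Hover, selection and path events set flags, then SetTileColor updates material parameters, brightening hovered tiles and turning path tiles blue.
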(event OnBeginCursorOver(Cube)
  (params (TouchedComponent :type Primitive%20Component%20Object%20Reference))
  (CallFunction|EventStartOverTile)
  (Default|EventNewTileOvered (Variables|Grid|Getbp_Grid) self))

(event OnEndCursorOver(Cube)
  (params (TouchedComponent :type Primitive%20Component%20Object%20Reference))
  (Default|EventNewTileOvered (Variables|Grid|Getbp_Grid)))

(event OnClicked(Cube)
  (params (TouchedComponent :type Primitive%20Component%20Object%20Reference) (ButtonPressed :type Key%20Structure :default "None"))
  (CallFunction|EventSelectTile)
  (Default|EventNewTileSelected (Variables|Grid|Getbp_Grid) self))

(event Custom|Event_DeselectTile
  (Variables|グリッド|SetblsSelected false)
  (CallFunction|SetTileColor))

(event Custom|Event_SelectTile
  (Variables|グリッド|SetblsSelected true)
  (CallFunction|SetTileColor))

(event Custom|Event_StartOverTile
  (Variables|Default|SetbIsOvered true)
  (CallFunction|SetTileColor))

(event Custom|Event_EndOverTile
  (Variables|Default|SetbIsOvered false)
  (CallFunction|SetTileColor))

(event Custom|Event_IsInPath
  (params (bIsInPath :type Boolean))
  (Variables|Default|SetbIsInPath bIsInPath)
  (CallFunction|SetTileColor))

(event EventBeginPlay
  (Utilities|FlowControl|Delay 0.2)
  (CallFunction|SetTileColor)
  (グリッド|SetTileSize)
  (Debug|SetWidgetVariables))

(fn ConstructionScript)

(fn SetTileColor
  (Utilities|FlowControl|Sequence
    (:then_0
      (switch Utilities|FlowControl|Switch|SwitchonEnum_GroundType (.groundtype (Grid|GetTileData))
        (:NewEnumerator0
          (LocalVariables|SetTileColor "(R=0.845772,G=1.000000,B=0.808946,A=1.000000)"))
        (:NewEnumerator1
          (LocalVariables|SetTileColor "(R=0.101052,G=0.712500,B=0.097559,A=1.000000)"))
        (:NewEnumerator2
          (LocalVariables|SetTileColor "(R=0.795833,G=0.328400,B=0.000000,A=1.000000)"))
        (:NewEnumerator3
          (LocalVariables|SetTileColor "(R=1.000000,G=0.000000,B=0.094805,A=1.000000)"))
        (:NewEnumerator4
          (LocalVariables|SetTileColor "(R=0.400000,G=0.400000,B=0.400000,A=1.000000)"))))
    (:then_1
      (if (Variables|グリッド|GetblsSelected)
        (Rendering|Material|SetScalarParameterValueonMaterials (Variables|Default|GetCube) "bIsSelected" 1.0)
        (else
          (Rendering|Material|SetScalarParameterValueonMaterials (Variables|Default|GetCube) "bIsSelected" 0.0))))
    (:then_2
      (if (Variables|Default|GetbIsOvered)
        (LocalVariables|SetTileColor (Math|Conversions|ToLinearColor(Vector) (* (Math|Conversions|ToVector(LinearColor) (LocalVariables|GetTileColor)) 3.0)))))
    (:then_3
      (if (Variables|Default|GetbIsInPath)
        (LocalVariables|SetTileColor "(R=0.000000,G=0.030910,B=1.000000,A=1.000000)")))
    (:then_4
      (Rendering|Material|SetVectorParameterValueonMaterials (Variables|Default|GetCube) "TileColor" (Math|Conversions|ToVector(LinearColor) (LocalVariables|GetTileColor))))))

(fn GetTileData
  (return (.Value (Utilities|Map|Find (Variables|/Game/Blueprint/Grid/BP_Grid.BP_Grid_C|Getstruct_Tiles (Variables|Grid|Getbp_Grid)) (Variables|Default|Getgridindex)))))

(fn SetTileSize
  (bind _bp_grid (Variables|Grid|Getbp_Grid))
  (bind _cube (Variables|Default|GetCube))
  (bind _returnvalue (Transformation|GetWorldScale _cube))
  (bind _tilesize (Variables|/Game/Blueprint/Grid/BP_Grid.BP_Grid_C|GetTileSize _bp_grid))
  (bind _returnvalue_2 (/ _tilesize 5e+01))
  (bind _returnvalue_3 (* _returnvalue _returnvalue_2))
  (Transformation|SetWorldScale3D (Variables|Default|GetCube) (Math|Vector|MakeVector (.x _returnvalue_3) (.y _returnvalue_3) 0.1)))

(fn SetWidgetVariables
  (bind _widget (Variables|Default|GetWidget))
  (bind _returnvalue (UserInterface|GetUserWidgetObject _widget))
  (bind _asw_grid_tile (Utilities|Casting|CastToW_GridTile _returnvalue))
  (Variables|/Game/Blueprint/Grid/W_GridTile.W_GridTile_C|Setgrid _asw_grid_tile (Variables|Grid|Getbp_Grid))
  (Variables|/Game/Blueprint/Grid/W_GridTile.W_GridTile_C|SetgridIndex _asw_grid_tile (Variables|Default|Getgridindex)))